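; SnowBoxBP is a trigger actor that fades tessellated snow on a sphere in and out as things enter and leave its box.
; The construction script creates a dynamic instance of the tessellated snow material, zeroes its SnowAmount parameter and applies it to the sphere.
; Box overlap plays the Snow timeline to drive SnowAmount, and end overlap reverses it.
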(event OnComponentBeginOverlap(Box)
  (params (OtherActor :type Actor%20Object%20Reference) (OtherComp :type Primitive%20Component%20Object%20Reference) (OtherBodyIndex :type Integer) (bFromSweep :type Boolean) (SweepResult :type Hit%20Result%20Structure%20%28by%20ref%29))
  (bind _newtrack_0 (Timeline|Snow Play)
    (:Update
      (Rendering|Material|SetScalarParameterValue (Variables|Default|GetSnowMaterialInstance) "SnowAmount" _newtrack_0 :!class /Script/Engine.MaterialInstanceDynamic))))

(event OnComponentEndOverlap(Box)
  (params (OtherActor :type Actor%20Object%20Reference) (OtherComp :type Primitive%20Component%20Object%20Reference) (OtherBodyIndex :type Integer))
  (bind _newtrack_0 (Timeline|Snow Reverse)
    (:Update
      (Rendering|Material|SetScalarParameterValue (Variables|Default|GetSnowMaterialInstance) "SnowAmount" _newtrack_0 :!class /Script/Engine.MaterialInstanceDynamic))))

(event EventBeginPlay)

(event EventActorBeginOverlap
  (params (OtherActor :type Actor%20Object%20Reference)))

(event EventTick
  (params (DeltaSeconds :type Float%20%28single-precision%29)))

(fn ConstructionScript
  (bind _returnvalue (Rendering|Material|CreateDynamicMaterialInstance "/Game/Tessellation/TessellatedSnowMaterial.TessellatedSnowMaterial" :!class /Script/Engine.KismetMaterialLibrary))
  (Variables|Default|SetSnowMaterialInstance _returnvalue)
  (Rendering|Material|SetScalarParameterValue (Variables|Default|GetSnowMaterialInstance) "SnowAmount" 0.0 :!class /Script/Engine.MaterialInstanceDynamic)
  (Rendering|Material|SetTextureParameterValue (Variables|Default|GetSnowMaterialInstance) "BasicTexture" 0)
  (Rendering|Material|SetMaterial (Variables|Default|GetSphere) 0 (Variables|Default|GetSnowMaterialInstance)))